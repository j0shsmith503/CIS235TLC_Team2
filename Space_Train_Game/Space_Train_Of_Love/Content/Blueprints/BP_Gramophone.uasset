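; Interactive gramophone that the first-person player can start and stop with E while inside its box trigger.
; Overlap enables or disables input on the actor and updates the HUD prompt to match the spinning state.
; Each toggle swaps the record material between static and spinning versions, activates or deactivates the audio, and calls BackgroundUpdate on the player character.
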(event `self.Box.OnComponentBeginOverlap`
  (params (OverlappedComponent :type "PrimitiveComponent Object Reference") (OtherActor :type "Actor Object Reference") (OtherComp :type "PrimitiveComponent Object Reference") (OtherBodyIndex :type Integer) (bFromSweep :type Boolean) (SweepResult :type "HitResult Structure (by ref)"))
  (bind _returnvalue (`PlayerController.GetHUD` (`GameplayStatics.GetPlayerController` 0)))
  (cast `/Game/FirstPerson/Blueprints/BP_FirstPersonCharacter` OtherActor)
  (set `self.isColliding` true)
  (`self.EnableInput` (`GameplayStatics.GetPlayerController` 0))
  (if (`self.isColliding`) :!label _label
    (bind _asnew_hud (cast `/Game/UI/NewHUD` _returnvalue))
    (if (`self.isSpinning`)
      (bind _asnew_hud_2 (cast `/Game/UI/NewHUD` (`PlayerController.GetHUD` (`GameplayStatics.GetPlayerController` 0))))
      (if (and (`self.isColliding`) (`self.isSpinning`))
        (set `/Game/UI/WB_HUD.Text` "'E' to stop" (`/Game/UI/NewHUD.UI Ref` _asnew_hud_2))
        (bind _ui_ref (`/Game/UI/NewHUD.UI Ref` _asnew_hud))
        (`/Game/UI/WB_HUD.UpdateText` _ui_ref :!label _label_2))
      (else
        (set `/Game/UI/WB_HUD.Text` "'E' to start" _ui_ref)
        (goto _label_2)))
    (else
      (bind _asnew_hud_3 (cast `/Game/UI/NewHUD` _returnvalue))
      (set `/Game/UI/WB_HUD.Text` "" (`/Game/UI/NewHUD.UI Ref` _asnew_hud_3))
      (goto _label_2))))

(event `self.Box.OnComponentEndOverlap`
  (params (OverlappedComponent :type "PrimitiveComponent Object Reference") (OtherActor :type "Actor Object Reference") (OtherComp :type "PrimitiveComponent Object Reference") (OtherBodyIndex :type Integer))
  (cast `/Game/FirstPerson/Blueprints/BP_FirstPersonCharacter` OtherActor)
  (set `self.isColliding` false)
  (`self.DisableInput` (`GameplayStatics.GetPlayerController` 0))
  (goto _label))

(event `Key|E`
  (params (Key :type "Key Structure"))
  (:`Pressed`
    (if (`self.isSpinning`)
      (`PrimitiveComponent.SetMaterial` (`self.SM_Gramaphone`) (`self.Element Index`) "/Game/Materials/M_Gramaphone_Record.M_Gramaphone_Record")
      (`|ExecutionSequence`
        (:`then_0`
          (set `self.isSpinning` false))
        (:`then_1`
          (bind _asbp_first_person_character (cast `/Game/FirstPerson/Blueprints/BP_FirstPersonCharacter` (`GameplayStatics.GetPlayerCharacter` 0)))
          (`/Game/FirstPerson/Blueprints/BP_FirstPersonCharacter.Background_Update` _asbp_first_person_character))
        (:`then_2`
          (`ActorComponent.Deactivate` (`self.Audio`))))
      (else
        (set `self.isSpinning` true)
        (`PrimitiveComponent.SetMaterial` (`self.SM_Gramaphone`) (`self.Element Index`) "/Game/Materials/M_Gramaphone_Record_Spinning.M_Gramaphone_Record_Spinning")
        (`|ExecutionSequence`
          (:`then_0`
            (bind _asbp_first_person_character_2 (cast `/Game/FirstPerson/Blueprints/BP_FirstPersonCharacter` (`GameplayStatics.GetPlayerCharacter` 0)))
            (`/Game/FirstPerson/Blueprints/BP_FirstPersonCharacter.Background_Update` _asbp_first_person_character_2))
          (:`then_1`
            (`ActorComponent.Activate` (`self.Audio`) false))))))
  (:`Released`
    (bind _asnew_hud (cast `/Game/UI/NewHUD` (`PlayerController.GetHUD` (`GameplayStatics.GetPlayerController` 0))))
    (if (and (`self.isColliding`) (`self.isSpinning`))
      (bind _ui_ref (`/Game/UI/NewHUD.UI Ref` _asnew_hud))
      (set `/Game/UI/WB_HUD.Text` " 'E' to stop" _ui_ref)
      (else
        (set `/Game/UI/WB_HUD.Text` "'E' to start" _ui_ref)))
    (`/Game/UI/WB_HUD.UpdateText` _ui_ref)))

(fn `UserConstructionScript`)