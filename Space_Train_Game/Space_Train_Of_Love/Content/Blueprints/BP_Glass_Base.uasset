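; Base glass window Blueprint that the player fades and unfades by pressing E while nearby.
; Collision overlap with the first-person character toggles input and the HUD prompt.
; Fading applies a dynamic M_Glass_Mirror instance and plays the FadeToClear timeline on Opacity; unfading swaps to M_Glass_Window and reverses it.
; The timeline's Finished output flips GlassFaded, which selects the next action.
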(event `Key|E`
  (params (Key :type "Key Structure"))
  (:`Pressed`
    (if (and (`self.Is Colliding Item`) (`self.GlassFaded`))
      (`self.Un_Fade`)
      (else
        (`self.Fade_Glass`)))))

(event `self.Collision.OnComponentBeginOverlap`
  (params (OverlappedComponent :type "PrimitiveComponent Object Reference") (OtherActor :type "Actor Object Reference") (OtherComp :type "PrimitiveComponent Object Reference") (OtherBodyIndex :type Integer) (bFromSweep :type Boolean) (SweepResult :type "HitResult Structure (by ref)"))
  (bind _returnvalue (`PlayerController.GetHUD` (`GameplayStatics.GetPlayerController` 0)))
  (cast `/Game/FirstPerson/Blueprints/BP_FirstPersonCharacter` OtherActor)
  (set `self.Is Colliding Item` true)
  (`self.EnableInput` (`GameplayStatics.GetPlayerController` 0))
  (if (`self.Is Colliding Item`) :!label _label
    (bind _asnew_hud (cast `/Game/UI/NewHUD` _returnvalue))
    (bind _ui_ref (`/Game/UI/NewHUD.UI Ref` _asnew_hud))
    (set `/Game/UI/WB_HUD.Text` "'E' to Fade" _ui_ref)
    (`/Game/UI/WB_HUD.UpdateText` _ui_ref)
    (else
      (bind _asnew_hud_2 (cast `/Game/UI/NewHUD` _returnvalue))
      (bind _ui_ref_2 (`/Game/UI/NewHUD.UI Ref` _asnew_hud_2))
      (set `/Game/UI/WB_HUD.Text` "" _ui_ref_2)
      (`/Game/UI/WB_HUD.UpdateText` _ui_ref_2))))

(event `self.Collision.OnComponentEndOverlap`
  (params (OverlappedComponent :type "PrimitiveComponent Object Reference") (OtherActor :type "Actor Object Reference") (OtherComp :type "PrimitiveComponent Object Reference") (OtherBodyIndex :type Integer))
  (cast `/Game/FirstPerson/Blueprints/BP_FirstPersonCharacter` OtherActor)
  (set `self.Is Colliding Item` false)
  (`self.DisableInput` (`GameplayStatics.GetPlayerController` 0))
  (goto _label))

(event `Fade_Glass`
  (bind _returnvalue (`KismetMaterialLibrary.CreateDynamicMaterialInstance` "/Game/Materials/M_Glass_Mirror.M_Glass_Mirror"))
  (bind _output_get (set `self.Temp Material` _returnvalue))
  (`PrimitiveComponent.SetMaterial` (`self.SM_GlassWindow`) 0 _output_get)
  (bind (_direction _fade_to_clear) (`Timeline|Fade to Clear` :!label _label_2)
    (:`Update`
      (`MaterialInstanceDynamic.SetScalarParameterValue` (`self.Temp Material`) (`self.Opacity`) _fade_to_clear))
    (:`Finished`
      (if (`self.GlassFaded`)
        (set `self.GlassFaded` false)
        (else
          (set `self.GlassFaded` true))))))

(event `Un_Fade`
  (bind _returnvalue (`KismetMaterialLibrary.CreateDynamicMaterialInstance` "/Game/Materials/M_Glass_Window.M_Glass_Window"))
  (bind _output_get (set `self.Temp Material` _returnvalue))
  (`PrimitiveComponent.SetMaterial` (`self.SM_GlassWindow`) 0 _output_get)
  (goto _label_2 :!via `Reverse`))

(fn `UserConstructionScript`)