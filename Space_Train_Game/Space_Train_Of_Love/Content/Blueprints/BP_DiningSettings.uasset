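; BP_DiningSettings is an interactable dining prop whose plate the player can shift and return with the E key.
; Box overlap with the first-person character toggles input and an "'E' to interact" prompt on NewHUD.
; E plays or reverses a timeline that offsets and rolls the plate, with an attached shifting sound.
; The ItemAlreadyMoved flag choosing the direction flips on every timeline update, rather than once on completion.
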(event `Key|E`
  (params (Key :type "Key Structure"))
  (:`Pressed`
    (if (and (`self.Is Colliding Item`) (`self.ItemAlreadyMoved`))
      (`self.Return_Items`)
      (else
        (`self.Move_Items`)))))

(event `self.Box.OnComponentBeginOverlap`
  (params (OverlappedComponent :type "PrimitiveComponent Object Reference") (OtherActor :type "Actor Object Reference") (OtherComp :type "PrimitiveComponent Object Reference") (OtherBodyIndex :type Integer) (bFromSweep :type Boolean) (SweepResult :type "HitResult Structure (by ref)"))
  (bind _returnvalue (`PlayerController.GetHUD` (`GameplayStatics.GetPlayerController` 0)))
  (cast `/Game/FirstPerson/Blueprints/BP_FirstPersonCharacter` OtherActor)
  (set `self.Is Colliding Item` true)
  (`self.EnableInput` (`GameplayStatics.GetPlayerController` 0))
  (if (`self.Is Colliding Item`) :!label _label
    (bind _asnew_hud (cast `/Game/UI/NewHUD` _returnvalue))
    (bind _ui_ref (`/Game/UI/NewHUD.UI Ref` _asnew_hud))
    (set `/Game/UI/WB_HUD.Text` "'E' to interact" _ui_ref)
    (`/Game/UI/WB_HUD.UpdateText` _ui_ref)
    (else
      (bind _asnew_hud_2 (cast `/Game/UI/NewHUD` _returnvalue))
      (bind _ui_ref_2 (`/Game/UI/NewHUD.UI Ref` _asnew_hud_2))
      (set `/Game/UI/WB_HUD.Text` "" _ui_ref_2)
      (`/Game/UI/WB_HUD.UpdateText` _ui_ref_2))))

(event `self.Box.OnComponentEndOverlap`
  (params (OverlappedComponent :type "PrimitiveComponent Object Reference") (OtherActor :type "Actor Object Reference") (OtherComp :type "PrimitiveComponent Object Reference") (OtherBodyIndex :type Integer))
  (cast `/Game/FirstPerson/Blueprints/BP_FirstPersonCharacter` OtherActor)
  (set `self.Is Colliding Item` false)
  (`self.DisableInput` (`GameplayStatics.GetPlayerController` 0))
  (goto _label))

(event `Move_Items`
  (`|ExecutionSequence`
    (:`then_0`
      (bind (_direction _plate_movement) (`Timeline|Plate_Movement` :!label _label_2)
        (:`Update`
          (`SceneComponent.K2_SetRelativeLocationAndRotation` (`self.Plate`) (`KismetMathLibrary.MakeVector` 0.0 (* _plate_movement 10.0) (* _plate_movement 15.0)) (`KismetMathLibrary.MakeRotator` (* _plate_movement 45.0)) false false)
          (if (`self.ItemAlreadyMoved`)
            (set `self.ItemAlreadyMoved` false)
            (else
              (set `self.ItemAlreadyMoved` true))))))
    (:`then_1`
      (`GameplayStatics.SpawnSoundAttached` "/Game/Sounds/Small_Item_Shift2.Small_Item_Shift2" (`self.Plate`) "None" (0.0 0.0 0.0) (struct) "KeepRelativeOffset" false 1.0 1.0 0.0 null null :!label _label_3))))

(event `Return_Items`
  (`|ExecutionSequence`
    (:`then_0`
      (goto _label_2 :!via `Reverse`))
    (:`then_1`
      (goto _label_3))))

(fn `UserConstructionScript`)