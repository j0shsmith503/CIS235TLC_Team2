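; Sliding double door that opens on E once the player has enough hearts for its door number, playing an acceptance or denial sound.
; Box overlap toggles input and shows or clears the HeartsNeeded text on the HUD.
; HeartCheck compares the character's CheckHearts result with a hardcoded threshold from DoorRequirements.
; Opening slides both panels apart on a Timeline, drops Collision out of the way and clears HeartsNeeded.
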(event `Key|E`
  (params (Key :type "Key Structure"))
  (bind _doorframe (`self.DoorFrame`))
  (:`Pressed`
    (bind _heartcheck (`self.HeartCheck` (`self.Door#`)))
    (if (and _heartcheck (`self.Is Colliding Item`))
      (`self.Open_Door`)
      (`GameplayStatics.SpawnSoundAttached` "/Game/Sounds/Terminal_Acceptance.Terminal_Acceptance" _doorframe "None" (0.0 0.0 0.0) (struct) "KeepRelativeOffset" false 1.0 1.0 0.0 null null)
      (else
        (`GameplayStatics.SpawnSoundAttached` "/Game/Sounds/Terminal_Denial.Terminal_Denial" _doorframe "None" (0.0 0.0 0.0) (struct) "KeepRelativeOffset" false 1.0 1.0 0.0 null null)))))

(event `self.Box.OnComponentBeginOverlap`
  (params (OverlappedComponent :type "PrimitiveComponent Object Reference") (OtherActor :type "Actor Object Reference") (OtherComp :type "PrimitiveComponent Object Reference") (OtherBodyIndex :type Integer) (bFromSweep :type Boolean) (SweepResult :type "HitResult Structure (by ref)"))
  (bind _returnvalue (`PlayerController.GetHUD` (`GameplayStatics.GetPlayerController` 0)))
  (cast `/Game/FirstPerson/Blueprints/BP_FirstPersonCharacter` OtherActor)
  (set `self.Is Colliding Item` true)
  (`self.EnableInput` (`GameplayStatics.GetPlayerController` 0))
  (if (`self.Is Colliding Item`) :!label _label
    (bind _asnew_hud (cast `/Game/UI/NewHUD` _returnvalue))
    (bind _ui_ref (`/Game/UI/NewHUD.UI Ref` _asnew_hud))
    (set `/Game/UI/WB_HUD.Text` (`self.Hearts Needed: `) _ui_ref)
    (`/Game/UI/WB_HUD.UpdateText` _ui_ref)
    (else
      (bind _asnew_hud_2 (cast `/Game/UI/NewHUD` _returnvalue))
      (bind _ui_ref_2 (`/Game/UI/NewHUD.UI Ref` _asnew_hud_2))
      (set `/Game/UI/WB_HUD.Text` "" _ui_ref_2)
      (`/Game/UI/WB_HUD.UpdateText` _ui_ref_2))))

(event `self.Box.OnComponentEndOverlap`
  (params (OverlappedComponent :type "PrimitiveComponent Object Reference") (OtherActor :type "Actor Object Reference") (OtherComp :type "PrimitiveComponent Object Reference") (OtherBodyIndex :type Integer))
  (cast `/Game/FirstPerson/Blueprints/BP_FirstPersonCharacter` OtherActor)
  (set `self.Is Colliding Item` false)
  (`self.DisableInput` (`GameplayStatics.GetPlayerController` 0))
  (goto _label))

(event `Open_Door`
  (`|ExecutionSequence`
    (:`then_0`
      (bind (_direction _door_movement) (`Timeline|Timeline`)
        (:`Update`
          (`|ExecutionSequence`
            (:`then_0`
              (`SceneComponent.K2_SetRelativeLocation` (`self.Door_L`) (`KismetMathLibrary.MakeVector` (* _door_movement -75.0)) false false)
              (set `self.ItemAlreadyMoved` false))
            (:`then_1`
              (`SceneComponent.K2_SetRelativeLocation` (`self.Door_R`) (`KismetMathLibrary.MakeVector` (* _door_movement 75.0)) false false)
              (set `self.Hearts Needed: ` "")
              (`SceneComponent.K2_SetRelativeLocation` (`self.Collision`) (0.0 0.0 -1000.0) false false))))))
    (:`then_1`
      (`GameplayStatics.SpawnSoundAttached` "/Game/Sounds/Door_Open.Door_Open" (`self.DoorFrame`) "None" (0.0 0.0 0.0) (struct) "KeepRelativeOffset" false 1.0 1.0 0.0 null null))))

(fn `DoorRequirements`
  (params (Door :type Integer))
  (returns (RequiredHearts :type Integer))
  (`|ExecutionSequence`
    (:`then_0`
      (bind _output_get (set `self.Door#` Door))
      (`/Engine/EditorBlueprintResources/StandardMacros.CompareInt` _output_get 1
        (:`==`
          (return 3))))
    (:`then_1`
      (bind _output_get_2 (set `self.Door#` Door))
      (`/Engine/EditorBlueprintResources/StandardMacros.CompareInt` _output_get_2 2
        (:`==`
          (return 6))))
    (:`then_2`
      (bind _output_get_3 (set `self.Door#` Door))
      (`/Engine/EditorBlueprintResources/StandardMacros.CompareInt` _output_get_3 3
        (:`==`
          (return 8))))
    (:`then_3`
      (bind _output_get_4 (set `self.Door#` Door))
      (`/Engine/EditorBlueprintResources/StandardMacros.CompareInt` _output_get_4 4
        (:`==`
          (return 12))))
    (:`then_4`
      (bind _output_get_5 (set `self.Door#` Door))
      (`/Engine/EditorBlueprintResources/StandardMacros.CompareInt` _output_get_5 5
        (:`==`
          (return 15))))))

(fn `HeartCheck`
  (params (Door :type Integer))
  (returns (HeartCheck :type Boolean))
  (`|ExecutionSequence`
    (:`then_0`
      (bind _asbp_first_person_character (cast `/Game/FirstPerson/Blueprints/BP_FirstPersonCharacter` (`GameplayStatics.GetPlayerCharacter` 0)))
      (bind _heartscollected (`/Game/FirstPerson/Blueprints/BP_FirstPersonCharacter.CheckHearts` _asbp_first_person_character)))
    (:`then_1`
      (bind _output_get (set `self.Door#` Door))
      (bind _requiredhearts (`self.DoorRequirements` _output_get))
      (`/Engine/EditorBlueprintResources/StandardMacros.CompareInt` _heartscollected _requiredhearts
        (:`>`
          _)
        (:`==`
          _))
      (return true))))

(fn `UserConstructionScript`)