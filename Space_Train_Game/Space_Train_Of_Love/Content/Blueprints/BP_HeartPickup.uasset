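; BP_HeartPickup is a heart collectible the first-person player picks up by pressing E.
; Sphere overlap with BP_FirstPersonCharacter toggles IsColliding and the actor's input, and shows or clears a prompt through NewHUD's UI widget.
; Pressing E in range notifies the UI via HeartFound, plays the pickup sound and animation, then destroys the actor after a short delay.
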(event `self.Sphere Collision.OnComponentBeginOverlap`
  (params (OverlappedComponent :type "PrimitiveComponent Object Reference") (OtherActor :type "Actor Object Reference") (OtherComp :type "PrimitiveComponent Object Reference") (OtherBodyIndex :type Integer) (bFromSweep :type Boolean) (SweepResult :type "HitResult Structure (by ref)"))
  (bind _returnvalue (`PlayerController.GetHUD` (`GameplayStatics.GetPlayerController` 0)))
  (cast `/Game/FirstPerson/Blueprints/BP_FirstPersonCharacter` OtherActor)
  (set `self.isColliding` true)
  (`self.EnableInput` (`GameplayStatics.GetPlayerController` 0))
  (if (`self.isColliding`) :!label _label
    (bind _asnew_hud (cast `/Game/UI/NewHUD` _returnvalue))
    (bind _ui_ref (`/Game/UI/NewHUD.UI Ref` _asnew_hud))
    (set `/Game/UI/WB_HUD.Text` "Press 'E' to pick up" _ui_ref)
    (`/Game/UI/WB_HUD.UpdateText` _ui_ref)
    (else
      (bind _asnew_hud_2 (cast `/Game/UI/NewHUD` _returnvalue))
      (bind _ui_ref_2 (`/Game/UI/NewHUD.UI Ref` _asnew_hud_2))
      (set `/Game/UI/WB_HUD.Text` "" _ui_ref_2)
      (`/Game/UI/WB_HUD.UpdateText` _ui_ref_2))))

(event `self.Sphere Collision.OnComponentEndOverlap`
  (params (OverlappedComponent :type "PrimitiveComponent Object Reference") (OtherActor :type "Actor Object Reference") (OtherComp :type "PrimitiveComponent Object Reference") (OtherBodyIndex :type Integer))
  (cast `/Game/FirstPerson/Blueprints/BP_FirstPersonCharacter` OtherActor)
  (set `self.isColliding` false)
  (`self.DisableInput` (`GameplayStatics.GetPlayerController` 0))
  (goto _label))

(event `Key|E`
  (params (Key :type "Key Structure"))
  (bind _heart_pickup (`self.Heart_Pickup`))
  (:`Pressed`
    (if (`self.isColliding`)
      (bind _asnew_hud (cast `/Game/UI/NewHUD` (`PlayerController.GetHUD` (`GameplayStatics.GetPlayerController` 0))))
      (`/Game/UI/WB_HUD.HeartFound` (`/Game/UI/NewHUD.UI Ref` _asnew_hud))
      (`GameplayStatics.SpawnSoundAttached` "/Game/Sounds/Heart_Pickup.Heart_Pickup" _heart_pickup "None" (0.0 0.0 0.0) (struct) "KeepRelativeOffset" false 1.0 1.0 0.0 null null)
      (`SkeletalMeshComponent.PlayAnimation` _heart_pickup "/Game/Animations/Heart_Pickup_Anim.Heart_Pickup_Anim" false)
      (`self.DestroyHeart`))))

(event `DestroyHeart`
  (`KismetSystemLibrary.Delay` 1.5)
  (`self.K2_DestroyActor`))

(fn `UserConstructionScript`)