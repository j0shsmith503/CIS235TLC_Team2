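; BP_ShutDownParticles is an actor that stages a train shutdown moment as soon as it begins play.
; It deactivates its dust Niagara component, then tints every Light actor in the level dark red and dims it.
; It then calls BackgroundUpdate on the first-person player character and plays the engine shut-down and train alarm sounds in 2D.
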(event `self.ReceiveBeginPlay`
  (`|ExecutionSequence`
    (:`then_0`
      (`ActorComponent.SetActive` (`self.NS_DustJCS`) false false)
      (bind _outactors (`GameplayStatics.GetAllActorsOfClass` "/Script/Engine.Light"))
      (for _array_element _outactors
        (`|ExecutionSequence`
          (:`then_0`
            (bind _lightcomponent (`Light.LightComponent` _array_element))
            (`LightComponent.SetLightColor` _lightcomponent (struct :`R` 0.307292 :`G` 0.011203 :`B` 0.015129 :`A` 1.0) true))
          (:`then_1`
            (`LightComponent.SetIntensity` _lightcomponent 0.1)))))
    (:`then_1`
      (bind _asbp_first_person_character (cast `/Game/FirstPerson/Blueprints/BP_FirstPersonCharacter` (`GameplayStatics.GetPlayerCharacter` 0)))
      (`/Game/FirstPerson/Blueprints/BP_FirstPersonCharacter.Background_Update` _asbp_first_person_character))
    (:`then_2`
      (`GameplayStatics.SpawnSound2D` "/Game/Sounds/Train_Engine_-_Shut_Down_BM.Train_Engine_-_Shut_Down_BM" 1.0 1.0 0.0 null))
    (:`then_3`
      (`GameplayStatics.SpawnSound2D` "/Game/Sounds/Train_Alarm.Train_Alarm" 1.0 1.0 0.0 null))))

(fn `UserConstructionScript`)