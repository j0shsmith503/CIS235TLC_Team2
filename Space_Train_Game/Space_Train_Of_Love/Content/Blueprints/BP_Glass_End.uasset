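; End-game glass window that fades clear when the player presses E in its trigger with at least 17 hearts.
; Trigger overlap toggles input and the HUD requirement text, and HeartCheck reads the character's count to pick the acceptance or denial sound.
; A timeline drives Opacity on a dynamic material instance.
; Its Finished branch sets GlassFaded, showing the delayed thanks message only if that flag was already set.
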(event `Key|E`
  (params (Key :type "Key Structure"))
  (bind _sm_glasswindow (`self.SM_GlassWindow`))
  (:`Pressed`
    (bind _heartcheck (`self.HeartCheck`))
    (if (and (`self.Is Colliding Item`) _heartcheck)
      (`self.Fade_Glass`)
      (`GameplayStatics.SpawnSoundAttached` "/Game/Sounds/Terminal_Acceptance.Terminal_Acceptance" _sm_glasswindow "None" (0.0 0.0 0.0) (struct) "KeepRelativeOffset" false 1.0 1.0 0.0 null null)
      (else
        (`GameplayStatics.SpawnSoundAttached` "/Game/Sounds/Terminal_Denial.Terminal_Denial" _sm_glasswindow "None" (0.0 0.0 0.0) (struct) "KeepRelativeOffset" false 1.0 1.0 0.0 null null)))))

(event `self.Collision.OnComponentBeginOverlap`
  (params (OverlappedComponent :type "PrimitiveComponent Object Reference") (OtherActor :type "Actor Object Reference") (OtherComp :type "PrimitiveComponent Object Reference") (OtherBodyIndex :type Integer) (bFromSweep :type Boolean) (SweepResult :type "HitResult Structure (by ref)"))
  (bind _returnvalue (`PlayerController.GetHUD` (`GameplayStatics.GetPlayerController` 0)))
  (cast `/Game/FirstPerson/Blueprints/BP_FirstPersonCharacter` OtherActor)
  (set `self.Is Colliding Item` true)
  (`self.EnableInput` (`GameplayStatics.GetPlayerController` 0))
  (if (`self.Is Colliding Item`) :!label _label
    (bind _asnew_hud (cast `/Game/UI/NewHUD` _returnvalue))
    (bind _ui_ref (`/Game/UI/NewHUD.UI Ref` _asnew_hud))
    (set `/Game/UI/WB_HUD.Text` "Hearts Needed: 17" _ui_ref)
    (`/Game/UI/WB_HUD.UpdateText` _ui_ref)
    (else
      (bind _asnew_hud_2 (cast `/Game/UI/NewHUD` _returnvalue))
      (bind _ui_ref_2 (`/Game/UI/NewHUD.UI Ref` _asnew_hud_2))
      (set `/Game/UI/WB_HUD.Text` "" _ui_ref_2)
      (`/Game/UI/WB_HUD.UpdateText` _ui_ref_2))))

(event `self.Collision.OnComponentEndOverlap`
  (params (OverlappedComponent :type "PrimitiveComponent Object Reference") (OtherActor :type "Actor Object Reference") (OtherComp :type "PrimitiveComponent Object Reference") (OtherBodyIndex :type Integer))
  (cast `/Game/FirstPerson/Blueprints/BP_FirstPersonCharacter` OtherActor)
  (set `self.Is Colliding Item` false)
  (`self.DisableInput` (`GameplayStatics.GetPlayerController` 0))
  (goto _label))

(event `Fade_Glass`
  (if (not (`self.GlassFaded`))
    (bind _returnvalue (`KismetMaterialLibrary.CreateDynamicMaterialInstance` "/Game/Materials/M_Glass_Mirror.M_Glass_Mirror"))
    (bind _output_get (set `self.Temp Material` _returnvalue))
    (`PrimitiveComponent.SetMaterial` (`self.SM_GlassWindow`) 0 _output_get)
    (bind (_direction _fade_to_clear) (`Timeline|Fade to Clear`)
      (:`Update`
        (`MaterialInstanceDynamic.SetScalarParameterValue` (`self.Temp Material`) (`self.Opacity`) _fade_to_clear))
      (:`Finished`
        (if (`self.GlassFaded`)
          (set `self.GlassFaded` false)
          (`KismetSystemLibrary.Delay` 5.0)
          (bind _asnew_hud (cast `/Game/UI/NewHUD` (`PlayerController.GetHUD` (`GameplayStatics.GetPlayerController` 0))))
          (bind _ui_ref (`/Game/UI/NewHUD.UI Ref` _asnew_hud))
          (set `/Game/UI/WB_HUD.Text` "Thanks for Playing!" _ui_ref)
          (`/Game/UI/WB_HUD.UpdateText` _ui_ref)
          (else
            (set `self.GlassFaded` true)))))))

(fn `HeartCheck`
  (returns (HeartCheck :type Boolean))
  (`|ExecutionSequence`
    (:`then_0`
      (bind _asbp_first_person_character (cast `/Game/FirstPerson/Blueprints/BP_FirstPersonCharacter` (`GameplayStatics.GetPlayerCharacter` 0)))
      (bind _heartscollected (`/Game/FirstPerson/Blueprints/BP_FirstPersonCharacter.CheckHearts` _asbp_first_person_character)))
    (:`then_1`
      (`/Engine/EditorBlueprintResources/StandardMacros.CompareInt` _heartscollected 17
        (:`>`
          _)
        (:`==`
          _))
      (return true))))

(fn `UserConstructionScript`)