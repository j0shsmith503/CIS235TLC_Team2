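; BP_Sink is an interactive sink that the player toggles on and off with E.
; A box overlap with the first-person character enables the actor's own input and shows an interact prompt through the NewHUD widget, reversing both on exit.
; Activation starts two RunningWater components and an attached looping sound, storing the sound reference so deactivation can stop it along with the water.
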(event `Key|E`
  (params (Key :type "Key Structure"))
  (:`Pressed`
    (if (and (`self.isColliding_Sink`) (`self.isSinkRunning`))
      (`self.DeactivateSink`)
      (else
        (`self.ActivateSink`)))))

(event `self.Box.OnComponentBeginOverlap`
  (params (OverlappedComponent :type "PrimitiveComponent Object Reference") (OtherActor :type "Actor Object Reference") (OtherComp :type "PrimitiveComponent Object Reference") (OtherBodyIndex :type Integer) (bFromSweep :type Boolean) (SweepResult :type "HitResult Structure (by ref)"))
  (bind _returnvalue (`PlayerController.GetHUD` (`GameplayStatics.GetPlayerController` 0)))
  (cast `/Game/FirstPerson/Blueprints/BP_FirstPersonCharacter` OtherActor)
  (set `self.isColliding_Sink` true)
  (`self.EnableInput` (`GameplayStatics.GetPlayerController` 0))
  (if (`self.isColliding_Sink`) :!label _label
    (bind _asnew_hud (cast `/Game/UI/NewHUD` _returnvalue))
    (bind _ui_ref (`/Game/UI/NewHUD.UI Ref` _asnew_hud))
    (set `/Game/UI/WB_HUD.Text` "'E' to interact" _ui_ref)
    (`/Game/UI/WB_HUD.UpdateText` _ui_ref)
    (else
      (bind _asnew_hud_2 (cast `/Game/UI/NewHUD` _returnvalue))
      (bind _ui_ref_2 (`/Game/UI/NewHUD.UI Ref` _asnew_hud_2))
      (set `/Game/UI/WB_HUD.Text` "" _ui_ref_2)
      (`/Game/UI/WB_HUD.UpdateText` _ui_ref_2))))

(event `self.Box.OnComponentEndOverlap`
  (params (OverlappedComponent :type "PrimitiveComponent Object Reference") (OtherActor :type "Actor Object Reference") (OtherComp :type "PrimitiveComponent Object Reference") (OtherBodyIndex :type Integer))
  (cast `/Game/FirstPerson/Blueprints/BP_FirstPersonCharacter` OtherActor)
  (set `self.isColliding_Sink` false)
  (`self.DisableInput` (`GameplayStatics.GetPlayerController` 0))
  (goto _label))

(event `ActivateSink`
  (`|ExecutionSequence`
    (:`then_0`
      (`ActorComponent.Activate` (`self.RunningWater1`) false)
      (set `self.isSinkRunning` true))
    (:`then_1`
      (`ActorComponent.Activate` (`self.RunningWater2`) false)
      (bind _returnvalue (`GameplayStatics.SpawnSoundAttached` "/Game/Sounds/Sink_Loop.Sink_Loop" (`self.Sink_0`) "None" (0.0 0.0 0.0) (struct) "KeepRelativeOffset" false 1.0 1.0 0.0 null null))
      (set `self.Sound` _returnvalue))))

(event `DeactivateSink`
  (bind _sound (`self.Sound`))
  (`|ExecutionSequence`
    (:`then_0`
      (`ActorComponent.Deactivate` (`self.RunningWater1`))
      (set `self.isSinkRunning` false)
      (if (`AudioComponent.IsPlaying` _sound)
        (`AudioComponent.Stop` _sound)))
    (:`then_1`
      (`ActorComponent.Deactivate` (`self.RunningWater2`)))))

(fn `UserConstructionScript`)